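; MenuController is a player controller that drives the front-end menu, moving between the splash screen and the main menu.
; On BeginPlay it finds the MainMenu widget; Enter starts the main menu, shows the cursor and centers it, while Backspace returns to the splash screen.
; A CanGoBack flag and two DoOnce gates that reset each other keep each transition from repeating until the opposite one has happened.
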(event `self.ReceiveBeginPlay`
  ;[0.6731 0.833 1] Get Menu Widget reference
  (bind _foundwidgets (`WidgetBlueprintLibrary.GetAllWidgetsOfClass` "/Game/IceAgeGame/Blueprints/UI_Widgets/MainMenu.MainMenu_C"))
  (set `self.menuScreen` (`|GetArrayItem` _foundwidgets) :!pinned true) ; Get reference to Menu UI
)

(event `Key|Enter`
  (params (Key :type "Key Structure"))
  (bind (_sizex _sizey) (`self.GetViewportSize`))
  ;[0.6731 0.833 1] Change Menu screen
  (:`Pressed`
    (`/Engine/EditorBlueprintResources/StandardMacros.DoOnce` true :!label _label
      (:`Completed`
        (`/Game/IceAgeGame/Blueprints/UI_Widgets/MainMenu.Start` (`self.menuScreen`)) ; Change to MainMenu
        (set `PlayerController.bShowMouseCursor` true (`GameplayStatics.GetPlayerController` 0))
        (`self.SetMouseLocation` (/ _sizex 2) (/ _sizey 2)) ; Center the mouse
        (set `self.canGoBack` true)
        (`self.ResetBack`)))))

(event `ResetStart`
  ;[0.6731 0.833 1] Change Menu screen
  (goto _label :!via `Reset`))

(event `Key|BackSpace`
  (params (Key :type "Key Structure"))
  ;[0.6731 0.833 1] Go back to splash screen (from main menu)
  (:`Pressed`
    (if (`self.canGoBack`)
      (set `self.canGoBack` false)
      (`/Engine/EditorBlueprintResources/StandardMacros.DoOnce` false :!label _label_2
        (:`Completed`
          (`/Game/IceAgeGame/Blueprints/UI_Widgets/MainMenu.GoBack` (`self.menuScreen`))
          (`self.ResetStart`))))))

(event `ResetBack`
  ;[0.6731 0.833 1] Go back to splash screen (from main menu)
  (goto _label_2 :!via `Reset`))

(fn `UserConstructionScript`)