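; GoldenAcorn is the level-ending collectible that Scrat picks up.
; It spins its root component by a fixed yaw every tick, so spin speed depends on frame rate.
; When a ScratTest overlaps the acorn, it plays a 3D collect sound through the level's SoundManager.
; It then calls FinishLevel on the FrozenRiver game mode and destroys itself.
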(event `self.ReceiveBeginPlay`
  ;[0.1198 0.1198 0.1198] Begin Play - Get player controller
  (bind _asscrat_controller (cast `/Game/IceAgeGame/Blueprints/Controller/ScratController` (`GameplayStatics.GetPlayerController` 0)))
  (set `self.Ctrl` _asscrat_controller)
  (bind _returnvalue (`GameplayStatics.GetActorOfClass` "/Game/IceAgeGame/Blueprints/WorldEntities/NotDisplayedEnt/SoundManager.SoundManager_C"))
  (set `self.Sound Manager` _returnvalue))

(event `self.ReceiveTick`
  (params (DeltaSeconds :type "Float (single-precision)"))
  ;[1 0.02034 0.1601] Event Tick
  (`self.Animate`))

(event `Animate`
  ;[1 0.5259 0.2611] Rotate the mesh
  (`SceneComponent.K2_AddLocalRotation` (`self.DefaultSceneRoot`) (struct :`Yaw` 1.5) false false))

(event `self.Acorn.OnComponentBeginOverlap`
  (params (OverlappedComponent :type "PrimitiveComponent Object Reference") (OtherActor :type "Actor Object Reference") (OtherComp :type "PrimitiveComponent Object Reference") (OtherBodyIndex :type Integer) (bFromSweep :type Boolean) (SweepResult :type "HitResult Structure (by ref)"))
  ;[0.2921 0.6108 1] If Scrat collects this particular nut, end the level and go back to the main menu
  (cast `/Game/IceAgeGame/Blueprints/Player/ScratTest` OtherActor)
  (`/Game/IceAgeGame/Blueprints/WorldEntities/NotDisplayedEnt/SoundManager.Play Sound 3D` (`self.Sound Manager`) "/Game/IceAgeGame/Sounds/SFX-Character/NutCollect.NutCollect" (`self.K2_GetActorLocation`))
  (bind _asfrozen_river (cast `/Game/IceAgeGame/Blueprints/GameModes/FrozenRiver` (`GameplayStatics.GetGameMode`)))
  (`/Game/IceAgeGame/Blueprints/GameModes/FrozenRiver.Finish Level` _asfrozen_river)
  (`self.K2_DestroyActor`))

(fn `UserConstructionScript`)