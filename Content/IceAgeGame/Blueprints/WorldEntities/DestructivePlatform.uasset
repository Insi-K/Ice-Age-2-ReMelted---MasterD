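; DestructivePlatform is an ice platform that slides along negative X and shatters when it reaches a Border.
; On BeginPlay it has a one-in-three chance to spawn an AcornToken at its Sphere, unless GoalSuccess is set.
; Tick moves it while Move is true and removes the token once GoalSuccess is set.
; Border overlap stops movement, damages the destructible mesh, destroys the token, then removes the actor after a delay.
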(event `self.ReceiveBeginPlay`
  (bind (_returnvalue_location _returnvalue_rotation) (`KismetMathLibrary.BreakTransform` (`SceneComponent.K2_GetComponentToWorld` (`self.Sphere`))))
  (if (and (== (`KismetMathLibrary.RandomInteger` 3) 1) (not (`self.GoalSuccess?`)))
    (bind _returnvalue (`|SpawnActorFromClass` "/Game/IceAgeGame/Blueprints/WorldEntities/AcornToken.AcornToken_C" (`KismetMathLibrary.MakeTransform` _returnvalue_location _returnvalue_rotation (1.5 1.5 1.5)) "AlwaysSpawn" "OverrideRootScale" null null))
    (set `/Game/IceAgeGame/Blueprints/WorldEntities/AcornToken.Location` (`self.Sphere`) _returnvalue)
    (set `self.Token` _returnvalue)))

(event `self.ReceiveTick`
  (params (DeltaSeconds :type "Float (single-precision)"))
  (bind _token (`self.Token`))
  (if (`self.Move`)
    (`self.K2_AddActorWorldOffset` (-2.5 0.0 0.0))
    (if (`self.GoalSuccess?`)
      (`/Engine/EditorBlueprintResources/StandardMacros.IsValid` _token
        (:`Is Valid`
          (`self.K2_DestroyActor` _token))))))

(event `self.PlatformCollision.OnComponentBeginOverlap`
  (params (OverlappedComponent :type "PrimitiveComponent Object Reference") (OtherActor :type "Actor Object Reference") (OtherComp :type "PrimitiveComponent Object Reference") (OtherBodyIndex :type Integer) (bFromSweep :type Boolean) (SweepResult :type "HitResult Structure (by ref)"))
  (bind _token (`self.Token`))
  (cast `/Game/IceAgeGame/Blueprints/WorldEntities/NotDisplayedEnt/Border` OtherActor)
  (set `self.Move` false)
  (`DestructibleComponent.ApplyDamage` (`self.IcePlatform_DM`) 100.0 (`SceneComponent.K2_GetComponentLocation` (`self.IcePlatform_DM`)) (0.0 0.0 0.0) 50.0)
  (`/Engine/EditorBlueprintResources/StandardMacros.IsValid` _token
    (:`Is Valid`
      (`self.K2_DestroyActor` _token))
    (:`Is Not Valid`
      _))
  (`KismetSystemLibrary.Delay` 3.0)
  (`self.K2_DestroyActor`))

(fn `UserConstructionScript`)