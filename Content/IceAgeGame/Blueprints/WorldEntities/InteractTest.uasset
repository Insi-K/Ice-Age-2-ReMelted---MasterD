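; InteractTest is a test interactable world actor that shows a hover text prompt when the ScratTest character enters its interaction area.
; Overlap begin and end set CanInteract and the Interactible reference on the ScratController, toggle the text, and open or close a gate.
; Every tick the text turns to face the camera, and while the gate is open it hides whenever InteractionStarted is true.
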(event `self.ReceiveTick`
  (params (DeltaSeconds :type "Float (single-precision)"))
  ;[0.2768 1 0.8598] Event Tick
  (`self.LookAtPlayer`)
  (`self.UpdateHoverText`))

(event `UpdateHoverText`
  (bind _display_text (`self.Display Text`))
  ;[1 1 1] Update visibility when interaction has started
  (`/Engine/EditorBlueprintResources/StandardMacros.Gate` true :!label _label
    (:`Exit`
      (if (`self.interactionStarted`)
        (`SceneComponent.SetVisibility` _display_text false false)
        (else
          (`SceneComponent.SetVisibility` _display_text true false))))))

(event `LookAtPlayer`
  ;[0.2768 1 0.8598] Update text rotation to look at player
  (`SceneComponent.K2_SetWorldRotation` (`self.Display Text`) (`KismetMathLibrary.FindLookAtRotation` (`self.K2_GetActorLocation`) (`PlayerCameraManager.GetCameraLocation` (`GameplayStatics.GetPlayerCameraManager` 0))) false false))

(event `OpenHover`
  ;[1 1 1] Update visibility when interaction has started
  (goto _label :!via `Open`))

(event `CloseHover`
  ;[1 1 1] Update visibility when interaction has started
  (goto _label :!via `Close`))

(event `self.InteractArea.OnComponentBeginOverlap`
  (params (OverlappedComponent :type "PrimitiveComponent Object Reference") (OtherActor :type "Actor Object Reference") (OtherComp :type "PrimitiveComponent Object Reference") (OtherBodyIndex :type Integer) (bFromSweep :type Boolean) (SweepResult :type "HitResult Structure (by ref)"))
  ;[0.6983 0.4166 1] Interaction Zone
  (bind _asscrat_test (cast `/Game/IceAgeGame/Blueprints/Player/ScratTest` OtherActor))
  (bind _asscrat_controller (cast `/Game/IceAgeGame/Blueprints/Controller/ScratController` (`Pawn.GetController` _asscrat_test)))
  (set `/Game/IceAgeGame/Blueprints/Controller/ScratController.canInteract` true _asscrat_controller)
  (`SceneComponent.SetVisibility` (`self.Display Text`) true false)
  (set `/Game/IceAgeGame/Blueprints/Controller/ScratController.Interactible` self _asscrat_controller)
  (`self.OpenHover`))

(event `self.InteractArea.OnComponentEndOverlap`
  (params (OverlappedComponent :type "PrimitiveComponent Object Reference") (OtherActor :type "Actor Object Reference") (OtherComp :type "PrimitiveComponent Object Reference") (OtherBodyIndex :type Integer))
  ;[0.6983 0.4166 1] Interaction Zone
  (bind _asscrat_test (cast `/Game/IceAgeGame/Blueprints/Player/ScratTest` OtherActor))
  (bind _asscrat_controller (cast `/Game/IceAgeGame/Blueprints/Controller/ScratController` (`Pawn.GetController` _asscrat_test)))
  (set `/Game/IceAgeGame/Blueprints/Controller/ScratController.canInteract` false _asscrat_controller)
  (`SceneComponent.SetVisibility` (`self.Display Text`) false false)
  (set `/Game/IceAgeGame/Blueprints/Controller/ScratController.Interactible` null _asscrat_controller)
  (`self.CloseHover`))

(fn `UserConstructionScript`)