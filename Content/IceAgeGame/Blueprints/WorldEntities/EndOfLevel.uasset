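; EndOfLevel is a level-exit trigger that marks whether the Scrat player is able to finish the level.
; When a ScratTest pawn enters or leaves its Box, it sets CanFinishLevel on that pawn's ScratController to true or false.
; BeginPlay caches player 0's ScratController, though the overlap events fetch the controller from the overlapping pawn instead.
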(event `self.ReceiveBeginPlay`
  ;[0.1198 0.1198 0.1198] Event Begin Play - Get references
  (bind _asscrat_controller (cast `/Game/IceAgeGame/Blueprints/Controller/ScratController` (`GameplayStatics.GetPlayerController` 0)))
  (set `self.As Scrat Controller` _asscrat_controller))

(event `self.Box.OnComponentBeginOverlap`
  (params (OverlappedComponent :type "PrimitiveComponent Object Reference") (OtherActor :type "Actor Object Reference") (OtherComp :type "PrimitiveComponent Object Reference") (OtherBodyIndex :type Integer) (bFromSweep :type Boolean) (SweepResult :type "HitResult Structure (by ref)"))
  ;[1 0.1406 0.1406] On Overlap - Display message on UI
  (bind _asscrat_test (cast `/Game/IceAgeGame/Blueprints/Player/ScratTest` OtherActor))
  (bind _asscrat_controller (cast `/Game/IceAgeGame/Blueprints/Controller/ScratController` (`Pawn.GetController` _asscrat_test)))
  (set `/Game/IceAgeGame/Blueprints/Controller/ScratController.canFinishLevel` true _asscrat_controller))

(event `self.Box.OnComponentEndOverlap`
  (params (OverlappedComponent :type "PrimitiveComponent Object Reference") (OtherActor :type "Actor Object Reference") (OtherComp :type "PrimitiveComponent Object Reference") (OtherBodyIndex :type Integer))
  ;[1 0.1406 0.1406] On Overlap - Display message on UI
  (bind _asscrat_test (cast `/Game/IceAgeGame/Blueprints/Player/ScratTest` OtherActor))
  (bind _asscrat_controller (cast `/Game/IceAgeGame/Blueprints/Controller/ScratController` (`Pawn.GetController` _asscrat_test)))
  (set `/Game/IceAgeGame/Blueprints/Controller/ScratController.canFinishLevel` false _asscrat_controller))

(fn `UserConstructionScript`)