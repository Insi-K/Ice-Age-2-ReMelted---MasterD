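; Scrat player character that adapts camera and water rules to the Main Game or Frozen River mode.
; Tick and landing update the jump permission on ScratController, enabling double jumps.
; Main Game water triggers game over; river water costs HP and bounces Scrat upward with a scream and slower movement.
; Repeated hits or depleted HP simulate freezing by swapping possession to a spawned ScratTest1 duplicate, flagged to restart when HP runs out.
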(event `Check Ground State`
  (bind _as_scrat_controller (`self.As Scrat Controller`))
  ;[1 0.1406 0.1406 1 72] In Gameplay
  ;;[1 1 1] Check Ground State
  (bind _output_get (set `self.isGrounded` (`NavMovementComponent.IsMovingOnGround` (`self.CharacterMovement`))))
  (if _output_get
    _
    (elif (`self.isJumping`)
      (set `/Game/IceAgeGame/Blueprints/Controller/ScratController.canJump` true _as_scrat_controller) ; This allows the player to perform a double jump
      (else
        (set `/Game/IceAgeGame/Blueprints/Controller/ScratController.canJump` false _as_scrat_controller) ; This prevents the player from jumping in certain states
      ))))

(event `self.OnLanded`
  (params (Hit :type "HitResult Structure (by ref)"))
  ;[1 0.1406 0.1406 1 72] In Gameplay
  ;;[0.4773 0.4267 1] Reset Ground-dependent variables
  (set `self.isJumping` false)
  (set `self.isSecondJump?` false)
  (set `/Game/IceAgeGame/Blueprints/Controller/ScratController.canJump` true (`self.As Scrat Controller`))
  (if (`self.RiverSensible`)
    (set `CharacterMovementComponent.MaxWalkSpeed` 800.0 (`self.CharacterMovement`))
    (set `self.FrozeCount` 0)
    (set `self.isFreezing?` false)))

(event `self.ReceivePossessed`
  (params (NewController :type "Controller Object Reference"))
  ;[0.06325 0.06771 0.06298 1 72] Basic Configuration
  ;;[0.4773 0.4267 1] Set up reference in controller
  (bind _asscrat_controller (cast `/Game/IceAgeGame/Blueprints/Controller/ScratController` NewController))
  (`/Game/IceAgeGame/Blueprints/Controller/ScratController.Set up possession` _asscrat_controller self)
  (`self.EnableInput` _asscrat_controller null)
  (set `/Game/IceAgeGame/Blueprints/Controller/ScratController.canJump` true _asscrat_controller))

(event `self.ReceiveTick`
  (params (DeltaSeconds :type "Float (single-precision)"))
  ;[0.06325 0.06771 0.06298 1 72] Basic Configuration
  ;;[0.4773 0.4267 1] Event Tick
  (`self.Check Ground State`))

(event `self.ReceiveBeginPlay`
  ;[0.06325 0.06771 0.06298 1 72] Basic Configuration
  ;;[1 1 1] Get References
  (bind _asscrat_controller (cast `/Game/IceAgeGame/Blueprints/Controller/ScratController` (`GameplayStatics.GetPlayerController` 0)))
  (bind _output_get (set `self.As Scrat Controller` _asscrat_controller))
  (set `/Game/IceAgeGame/Blueprints/Controller/ScratController.canJump` true _output_get) ; Allow the player to jump from start
)

(event `Player Setup`
  (params (`Current Game Mode` :type "/Game/IceAgeGame/GameMode Enum" :default "NewEnumerator0"))
  ;[0.06325 0.06771 0.06298 1 72] Basic Configuration
  ;;[1 1 1] Player Setup - Prepare the character to work different depending on the current game mode in level
  (switch `/Game/IceAgeGame/GameMode` `Current Game Mode`
    (:`NewEnumerator0`
      (`ActorComponent.Activate` (`self.MainCam`) false)
      (set `self.WaterIntolerant` true))
    (:`NewEnumerator1`
      (`ActorComponent.Activate` (`self.MainRiverCam`) false)
      (set `self.RiverSensible` true)
      (bind _asfrozen_river (cast `/Game/IceAgeGame/Blueprints/GameModes/FrozenRiver` (`GameplayStatics.GetGameMode`)))
      (set `/Game/IceAgeGame/Blueprints/GameModes/FrozenRiver.Spawn` (`self.K2_GetActorLocation`) _asfrozen_river))))

(event `self.Sphere.OnComponentBeginOverlap`
  (params (OverlappedComponent :type "PrimitiveComponent Object Reference") (OtherActor :type "Actor Object Reference") (OtherComp :type "PrimitiveComponent Object Reference") (OtherBodyIndex :type Integer) (bFromSweep :type Boolean) (SweepResult :type "HitResult Structure (by ref)"))
  ;[1 0.5259 0.2611 1 72] Main Game - Work in progress
  ;;[1 1 1] Main Game - If player falls into water, then restart the level
  (cast `WaterBodyLake` OtherActor)
  (if (`self.WaterIntolerant`)
    (bind _asmain_game (cast `/Game/IceAgeGame/Blueprints/GameModes/MainGame` (`GameplayStatics.GetGameMode`)))
    (`/Game/IceAgeGame/Blueprints/GameModes/MainGame.Game Over` _asmain_game)
    (`Controller.UnPossess` (`self.As Scrat Controller`))
    (`self.K2_DestroyActor`)))

(event `self.CapsuleComponent.OnComponentBeginOverlap`
  (params (OverlappedComponent :type "PrimitiveComponent Object Reference") (OtherActor :type "Actor Object Reference") (OtherComp :type "PrimitiveComponent Object Reference") (OtherBodyIndex :type Integer) (bFromSweep :type Boolean) (SweepResult :type "HitResult Structure (by ref)"))
  (bind (_returnvalue_x _returnvalue_y _returnvalue_z) (`KismetMathLibrary.BreakVector` (`self.GetVelocity`)))
  (bind _charactermovement (`self.CharacterMovement`))
  (bind _as_scrat_controller (`self.As Scrat Controller`))
  (bind _as_scrat_controller_2 (`self.As Scrat Controller`))
  (bind _hp (`/Game/IceAgeGame/Blueprints/Controller/ScratController.hp` _as_scrat_controller_2))
  (bind _returnvalue (<= _hp 1))
  ;[0.2921 0.6108 1 1 72] Frozen River
  ;;[1 1 1] Frozen River - Jump Scream: If character has contact with the water, he will loose HP - If triggered 4 times in a row "Freeze" the character
  (cast `WaterBodyLake` OtherActor)
  (if (`self.RiverSensible`)
    (set `self.isFreezing?` true)
    (set `self.isJumping` false)
    (if (> (`self.FrozeCount`) 2)
      (if _returnvalue
        (set `/Game/IceAgeGame/Blueprints/Controller/ScratController.hp` 0 _as_scrat_controller_2 :!label _label) ; Set HP to 0
        (`self.Freeze` true)
        (else
          (`/Engine/EditorBlueprintResources/StandardMacros.DecrementInt` _hp ; Reduce HP by 1
            (:`  `
              (`self.Freeze` false)))))
      (elif _returnvalue
        (goto _label)
        (else
          (if (< _returnvalue_z -1000.0)
            (`CharacterMovementComponent.AddImpulse` _charactermovement (0.0 0.0 3400.0) true)
            (else
              (`CharacterMovementComponent.AddImpulse` _charactermovement (0.0 0.0 2000.0) true)))
          (`self.Scream`) ; Play SFX
          (set `CharacterMovementComponent.MaxWalkSpeed` 550.0 (`self.CharacterMovement`)) ; Player will move slower in the air
          (`/Engine/EditorBlueprintResources/StandardMacros.IncrementInt` (`self.FrozeCount`) ; Increase Froze Count
            (:`  `
              (`/Engine/EditorBlueprintResources/StandardMacros.DecrementInt` (`/Game/IceAgeGame/Blueprints/Controller/ScratController.hp` _as_scrat_controller) ; Reduce the HP by 1
                (:`  `
                  (set `/Game/IceAgeGame/Blueprints/Controller/ScratController.canJump` false _as_scrat_controller) ; Player will not be able to jump during this state
                  (`KismetSystemLibrary.Delay` 0.1)
                  (set `self.isFreezing?` false) ; Variable control for AnimBP
                )))))))))

(event `Freeze`
  (params (`Game Over?` :type Boolean))
  ;[0.2921 0.6108 1 1 72] Frozen River
  ;;[1 1 1] Freeze - Spawn character "duplicate" with no functionality and possess it (This simulates the player getting frozen in the water)
  (bind _asscrat_controller (cast `/Game/IceAgeGame/Blueprints/Controller/ScratController` (`self.GetController`)))
  (`self.DisableInput` _asscrat_controller null) ; When player is frozen - No input will be accepted
  (bind _returnvalue (`|SpawnActorFromClass` "/Game/IceAgeGame/Blueprints/Player/ScratTest1.ScratTest1_C" (`self.GetTransform`) "Undefined" "OverrideRootScale" null `Game Over?` null))
  (bind _asscrat_controller_2 (cast `/Game/IceAgeGame/Blueprints/Controller/ScratController` (`GameplayStatics.GetPlayerController` 0)))
  (`Controller.Possess` _asscrat_controller_2 _returnvalue)
  (`self.K2_DestroyActor`))

(event `Scream`
  ;[0.2921 0.6108 1 1 72] Frozen River
  ;;[1 1 1] Play frozen water SFX and Character scream
  (bind _returnvalue (`GameplayStatics.GetActorOfClass` "/Game/IceAgeGame/Blueprints/WorldEntities/NotDisplayedEnt/SoundManager.SoundManager_C"))
  (`/Game/IceAgeGame/Blueprints/WorldEntities/NotDisplayedEnt/SoundManager.Play Sound 3D` _returnvalue "/Game/IceAgeGame/Sounds/SFX-Character/River_1_Cue.River_1_Cue" (`self.K2_GetActorLocation`))
  (`/Game/IceAgeGame/Blueprints/WorldEntities/NotDisplayedEnt/SoundManager.Play Sound` _returnvalue "/Game/IceAgeGame/Sounds/SFX-Character/Scream1_Cue.Scream1_Cue"))

(fn `UserConstructionScript`)