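; MainGame is the game mode for the Ice Age game, handling game over, level restart and level completion for the Scrat player.
; It caches the ScratController on BeginPlay; GameOver stops music, disables input and, after a delay, restarts the level.
; Restart and finish fade out the PlayerUI widget before reopening the current level or loading MainMenuTest.
; SpawnPlayertoMap forwards player spawning through a call meant for the persistent map.
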(event `self.ReceiveBeginPlay`
  ;[0.1198 0.1198 0.1198] Get References
  (bind _asscrat_controller (cast `/Game/IceAgeGame/Blueprints/Controller/ScratController` (`GameplayStatics.GetPlayerController` 0)))
  (set `self.As Scrat Controller` _asscrat_controller))

(event `Game Over`
  ;[1 0.1406 0.1406] Play Game Over Screen and restart level
  (bind _returnvalue (`GameplayStatics.GetActorOfClass` "/Game/IceAgeGame/Blueprints/WorldEntities/NotDisplayedEnt/SoundManager.SoundManager_C"))
  (`/Game/IceAgeGame/Blueprints/WorldEntities/NotDisplayedEnt/SoundManager.Stop Music` _returnvalue 0.0)
  (`self.DisableInput` (`self.As Scrat Controller`) null)
  (`KismetSystemLibrary.Delay` 1.0)
  (`self.Restart Level`))

(event `Restart Level`
  ;[1 0.5259 0.2611] Restart the level
  (bind _foundwidgets (`WidgetBlueprintLibrary.GetAllWidgetsOfClass` "/Game/IceAgeGame/Blueprints/UI_Widgets/PlayerUI.PlayerUI_C" false))
  (`/Game/IceAgeGame/Blueprints/UI_Widgets/PlayerUI.ScreenFadeOut` (`|GetArrayItem` _foundwidgets))
  (`KismetSystemLibrary.Delay` 1.0)
  (bind _returnvalue (`GameplayStatics.GetCurrentLevelName` true))
  (`GameplayStatics.OpenLevel` (`KismetStringLibrary.Conv_StringToName` _returnvalue)))

(event `Spawn Player to Map`
  ;[1 0.3338 0.06105] Make call to Event in Persistent Map
  (`self.Call Spawn Player`))

(event `Finish Level`
  ;[0.5684 0.3165 1] Finish Level - Goes Back to Main Menu
  (bind _foundwidgets (`WidgetBlueprintLibrary.GetAllWidgetsOfClass` "/Game/IceAgeGame/Blueprints/UI_Widgets/PlayerUI.PlayerUI_C" false))
  (`/Game/IceAgeGame/Blueprints/UI_Widgets/PlayerUI.ScreenFadeOut` (`|GetArrayItem` _foundwidgets))
  (`KismetSystemLibrary.Delay` 2.0)
  (`GameplayStatics.OpenLevel` "MainMenuTest"))

(fn `UserConstructionScript`)