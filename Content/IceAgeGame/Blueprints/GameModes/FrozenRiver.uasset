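; Game mode for the Frozen River level that runs the acorn token goal, player respawns, level restarts and the finish.
; Tick polls the controller's token count; at 20 it fades out, calls the Golden Acorn spawn, flags DestructivePlatforms and returns the player to start.
; Respawning possesses a newly spawned Scrat and reduces tokens, passing the goal flag.
; Win and lose sequences chain SoundManager cues, delays and PlayerUI fades, ending in respawn, level reload or main menu.
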(event `Set Goal Success`
  ;[0.5684 0.3165 1] Goal Success - Tells all the platforms in the level to remove the Acorn Tokens (This does not affect the Golden Token)
  (set `self.Goal Success?` true)
  (bind _outactors (`GameplayStatics.GetAllActorsOfClass` "/Game/IceAgeGame/Blueprints/WorldEntities/DestructivePlatform.DestructivePlatform_C"))
  (for _array_element _outactors
    (set `/Game/IceAgeGame/Blueprints/WorldEntities/DestructivePlatform.GoalSuccess?` true _array_element)))

(event `self.ReceiveBeginPlay`
  ;[0.1198 0.1198 0.1198] Event Begin Play - Get References
  (bind _asscrat_controller (cast `/Game/IceAgeGame/Blueprints/Controller/ScratController` (`GameplayStatics.GetPlayerController` 0)))
  (set `self.As Scrat Controller` _asscrat_controller))

(event `self.ReceiveTick`
  (params (DeltaSeconds :type "Float (single-precision)"))
  ;[1 0.02034 0.1601] Event Tick
  (`self.Check Goal Success`))

(event `Check Goal Success`
  (bind _as_scrat_controller (`self.As Scrat Controller`))
  ;[1 0.1406 0.1406] Core Game Mode Mechanic - Constantly check whether the player reaches the goal. When this is true, reset the player's position and spawn the Golden Token
  (if (== (`/Game/IceAgeGame/Blueprints/Controller/ScratController.nutTokens` _as_scrat_controller) 20)
    (`/Engine/EditorBlueprintResources/StandardMacros.DoOnce` false
      (:`Completed`
        (`/Game/IceAgeGame/Blueprints/Controller/ScratController.Stop Movement` _as_scrat_controller)
        (bind _foundwidgets (`WidgetBlueprintLibrary.GetAllWidgetsOfClass` "/Game/IceAgeGame/Blueprints/UI_Widgets/PlayerUI.PlayerUI_C" false))
        (bind _output (`|GetArrayItem` _foundwidgets))
        (`/Game/IceAgeGame/Blueprints/UI_Widgets/PlayerUI.ScreenFadeOut` _output)
        (bind _returnvalue (`GameplayStatics.GetActorOfClass` "/Game/IceAgeGame/Blueprints/WorldEntities/NotDisplayedEnt/SoundManager.SoundManager_C"))
        (`/Game/IceAgeGame/Blueprints/WorldEntities/NotDisplayedEnt/SoundManager.Stop Music` _returnvalue 0.0)
        (`/Game/IceAgeGame/Blueprints/WorldEntities/NotDisplayedEnt/SoundManager.Play Sound` _returnvalue "/Game/IceAgeGame/Sounds/RiverWin1.RiverWin1")
        (`KismetSystemLibrary.Delay` 4.0)
        (`self.SpawnGoldenAcorn`)
        (`self.Set Goal Success`)
        (`/Game/IceAgeGame/Blueprints/Controller/ScratController.BackToStart` (`self.As Scrat Controller`) (`self.Spawn`))
        (`/Game/IceAgeGame/Blueprints/UI_Widgets/PlayerUI.RiverFadeIn` _output)))))

(event `Restart Player`
  ;[0.2921 0.6108 1] Restart Player - This event simulates a certain animation scene by spawning a new player with no input temporarily and resets the player's position to the start location
  (bind _returnvalue (`GameplayStatics.GetActorOfClass` "/Game/IceAgeGame/Blueprints/WorldEntities/NotDisplayedEnt/SoundManager.SoundManager_C"))
  (`/Game/IceAgeGame/Blueprints/WorldEntities/NotDisplayedEnt/SoundManager.Stop Music` _returnvalue 0.0)
  (`self.DisableInput` (`self.As Scrat Controller`) null)
  (`KismetSystemLibrary.Delay` 0.5)
  (`/Game/IceAgeGame/Blueprints/WorldEntities/NotDisplayedEnt/SoundManager.Play Sound` _returnvalue "/Game/IceAgeGame/Sounds/RiverLoose.RiverLoose")
  (`KismetSystemLibrary.Delay` 3.0)
  (bind _foundwidgets (`WidgetBlueprintLibrary.GetAllWidgetsOfClass` "/Game/IceAgeGame/Blueprints/UI_Widgets/PlayerUI.PlayerUI_C"))
  (bind _output (`|GetArrayItem` _foundwidgets))
  (`/Game/IceAgeGame/Blueprints/UI_Widgets/PlayerUI.ScreenFadeOut` _output)
  (`KismetSystemLibrary.Delay` 0.5)
  (bind _returnvalue_2 (`|SpawnActorFromClass` "/Game/IceAgeGame/Blueprints/Player/ScratTest.ScratTest_C" (`KismetMathLibrary.MakeTransform` (`self.Spawn`)) "Undefined" "OverrideRootScale" null null))
  (`/Game/IceAgeGame/Blueprints/Player/ScratTest.Player Setup` _returnvalue_2 "NewEnumerator1")
  (`Controller.Possess` (`self.As Scrat Controller`) _returnvalue_2)
  (bind _returnvalue_3 (`GameplayStatics.GetActorOfClass` "/Game/IceAgeGame/Blueprints/Player/ScratTest1.ScratTest1_C"))
  (`self.K2_DestroyActor` _returnvalue_3)
  (`/Game/IceAgeGame/Blueprints/Controller/ScratController.ReduceTokens` (`self.As Scrat Controller`) (`self.Goal Success?`)) ; Only reduce tokens while goal is not completed
  (`/Game/IceAgeGame/Blueprints/UI_Widgets/PlayerUI.RiverFadeIn` _output))

(event `Restart`
  ;[0.2921 0.6108 1] If player HP is 0, Restart the level
  (bind _returnvalue (`GameplayStatics.GetActorOfClass` "/Game/IceAgeGame/Blueprints/WorldEntities/NotDisplayedEnt/SoundManager.SoundManager_C"))
  (`/Game/IceAgeGame/Blueprints/WorldEntities/NotDisplayedEnt/SoundManager.Stop Music` _returnvalue 0.0)
  (`self.DisableInput` (`self.As Scrat Controller`) null)
  (`KismetSystemLibrary.Delay` 0.5)
  (`/Game/IceAgeGame/Blueprints/WorldEntities/NotDisplayedEnt/SoundManager.Play Sound` _returnvalue "/Game/IceAgeGame/Sounds/RiverLoose.RiverLoose")
  (`KismetSystemLibrary.Delay` 3.0)
  (`self.Restart Level`))

(event `Spawn Player to Map`
  ;[1 0.3338 0.06105] Make call to Event in Persistent Map
  (`self.Spawn Player`))

(event `Finish Level`
  ;[0.5684 0.3165 1] End the level and Open the Main Menu
  (bind _returnvalue (`GameplayStatics.GetActorOfClass` "/Game/IceAgeGame/Blueprints/WorldEntities/NotDisplayedEnt/SoundManager.SoundManager_C"))
  (`/Game/IceAgeGame/Blueprints/WorldEntities/NotDisplayedEnt/SoundManager.Stop Music` _returnvalue 0.0)
  (`self.DisableInput` (`self.As Scrat Controller`) null)
  (`KismetSystemLibrary.Delay` 0.5)
  (`/Game/IceAgeGame/Blueprints/WorldEntities/NotDisplayedEnt/SoundManager.Play Sound` _returnvalue "/Game/IceAgeGame/Sounds/RiverWin2.RiverWin2")
  (`KismetSystemLibrary.Delay` 1.5)
  (bind _foundwidgets (`WidgetBlueprintLibrary.GetAllWidgetsOfClass` "/Game/IceAgeGame/Blueprints/UI_Widgets/PlayerUI.PlayerUI_C"))
  (`/Game/IceAgeGame/Blueprints/UI_Widgets/PlayerUI.ScreenFadeOut` (`|GetArrayItem` _foundwidgets))
  (`KismetSystemLibrary.Delay` 3.0)
  (`GameplayStatics.OpenLevel` "MainMenuTest"))

(event `Restart Level`
  ;[1 0.5259 0.2611] Restart the level
  (bind _foundwidgets (`WidgetBlueprintLibrary.GetAllWidgetsOfClass` "/Game/IceAgeGame/Blueprints/UI_Widgets/PlayerUI.PlayerUI_C"))
  (`/Game/IceAgeGame/Blueprints/UI_Widgets/PlayerUI.ScreenFadeOut` (`|GetArrayItem` _foundwidgets))
  (`KismetSystemLibrary.Delay` 1.0)
  (bind _returnvalue (`GameplayStatics.GetCurrentLevelName` true))
  (`GameplayStatics.OpenLevel` (`KismetStringLibrary.Conv_StringToName` _returnvalue)))

(fn `UserConstructionScript`)